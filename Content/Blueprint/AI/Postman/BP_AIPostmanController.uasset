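; AI controller for the postman that tracks whether a delivery is active.
; On BeginPlay it binds to the first-person game mode's delivery status event and caches the flag.
; GetMoveLocation uses that flag to return either the game mode's delivery point or the postman's home point.
; CreatePacket spawns a BP_Pickup at a given component's location and has the pickup ability attach it there as the carried object.
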(event `self.ReceiveBeginPlay`
  (`parent.ReceiveBeginPlay`)
  (bind _asfirst_person_game_mode (cast `/Game/FirstPersonBP/Blueprints/FirstPersonGameMode` (`GameplayStatics.GetGameMode`)))
  (add `/Game/FirstPersonBP/Blueprints/FirstPersonGameMode.OnDeliveryStatusChanged` _asfirst_person_game_mode (delegate `DeliveryStatusChanged`)))

(event `DeliveryStatusChanged`
  (params (IsDelivery :type Boolean))
  (set `self.IsDeliver` IsDelivery))

(fn `CreatePacket`
  (params (Parent :type "SceneComponent Object Reference"))
  (bind _returnvalue (`|SpawnActorFromClass` "/Game/Blueprint/Pickup/BP_Pickup.BP_Pickup_C" (`KismetMathLibrary.Conv_VectorToTransform` (`SceneComponent.K2_GetComponentLocation` Parent)) "Undefined" "OverrideRootScale" null null))
  (`/Game/Blueprint/Pickup/BPC_PickupAbility.Pickup Object` (`self.BP_PickupAbility`) _returnvalue Parent))

(fn `GetMoveLocation`
  (returns (Location :type "Vector Structure"))
  (bind _asfirst_person_game_mode (cast `/Game/FirstPersonBP/Blueprints/FirstPersonGameMode` (`GameplayStatics.GetGameMode`)))
  (if (`self.IsDeliver`)
    (return (`/Game/FirstPersonBP/Blueprints/FirstPersonGameMode.DeliveryPoint` _asfirst_person_game_mode))
    (else
      (return (`/Game/FirstPersonBP/Blueprints/FirstPersonGameMode.PostmanHomePoint` _asfirst_person_game_mode)))))

(fn `UserConstructionScript`
  (`parent.UserConstructionScript`))