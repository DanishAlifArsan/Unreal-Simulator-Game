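; AI controller for a customer NPC that moves between the cashier and its home point based on whether an order is active.
; On BeginPlay it subscribes to the game mode's order-status event and mirrors it into the IsOrder blackboard key.
; GetMoveLocation reads that key to return the game mode's CashierPoint or CustomerHomePoint.
; When the first-person player interacts with its pawn, it sets the game mode's order to false.
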(event `self.ReceiveBeginPlay`
  (`parent.ReceiveBeginPlay`)
  (bind _asfirst_person_game_mode (cast `/Game/FirstPersonBP/Blueprints/FirstPersonGameMode` (`GameplayStatics.GetGameMode`)))
  (add `/Game/FirstPersonBP/Blueprints/FirstPersonGameMode.OnOrderStatusChanged` _asfirst_person_game_mode (delegate `OnOrderChanged`))
  (`self.BindInteractEvent`))

(event `OnOrderChanged`
  (params (IsOrder :type Boolean))
  (`BlackboardComponent.SetValueAsBool` (`self.Blackboard`) "IsOrder" IsOrder))

(event `BindInteractEvent`
  (bind _asthird_person_character (cast `/Game/ThirdPersonBP/Blueprints/ThirdPersonCharacter` (`self.K2_GetPawn`)))
  (add `/Game/ThirdPersonBP/Blueprints/ThirdPersonCharacter.OnInteractEvent` _asthird_person_character (delegate `OnInteract`)))

(event `OnInteract`
  (params (Source :type "/Game/Blueprint/Interactable/BPC_InteractAbility Object Reference"))
  (cast `/Game/FirstPersonBP/Blueprints/FirstPersonCharacter` (`ActorComponent.GetOwner` Source))
  (bind _asfirst_person_game_mode (cast `/Game/FirstPersonBP/Blueprints/FirstPersonGameMode` (`GameplayStatics.GetGameMode`)))
  (`/Game/FirstPersonBP/Blueprints/FirstPersonGameMode.SetOrder` _asfirst_person_game_mode false))

(fn `GetMoveLocation`
  (returns (Location :type "Vector Structure"))
  (bind _asfirst_person_game_mode (cast `/Game/FirstPersonBP/Blueprints/FirstPersonGameMode` (`GameplayStatics.GetGameMode`)))
  (if (`BlackboardComponent.GetValueAsBool` (`self.Blackboard`) "IsOrder")
    (return (`/Game/FirstPersonBP/Blueprints/FirstPersonGameMode.CashierPoint` _asfirst_person_game_mode))
    (else
      (return (`/Game/FirstPersonBP/Blueprints/FirstPersonGameMode.CustomerHomePoint` _asfirst_person_game_mode)))))

(fn `UserConstructionScript`
  (`parent.UserConstructionScript`))