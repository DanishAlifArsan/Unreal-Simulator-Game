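; Component that lets its owner pick up and place physics objects.
; PickupObject skips objects already flagged as picked, otherwise stores the reference, snaps the object's Cube to the pickup point, attaches it and disables physics and collision.
; PlaceObject clears the flag, detaches the Cube at its current world transform, restores physics and collision, and clears the stored reference.
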(fn `Pickup Object`
  (params (PickedObject :type "/Game/Blueprint/Pickup/BP_Pickup Object Reference") (PickupPoint :type "SceneComponent Object Reference"))
  (if (`/Game/Blueprint/Pickup/BP_Pickup.IsPicked` PickedObject)
    (return)
    (else
      (bind _output_get (set `self.PickedObject` PickedObject))
      (set `/Game/Blueprint/Pickup/BP_Pickup.IsPicked` true _output_get)
      (bind _cube (`/Game/Blueprint/Pickup/BP_Pickup.Cube` _output_get))
      (`SceneComponent.K2_SetWorldLocation` _cube (`SceneComponent.K2_GetComponentLocation` PickupPoint) false false)
      (`SceneComponent.K2_AttachToComponent` _cube PickupPoint "None" "KeepWorld" "KeepWorld" "KeepWorld" true)
      (`PrimitiveComponent.SetSimulatePhysics` _cube false)
      (`PrimitiveComponent.SetCollisionEnabled` _cube "NoCollision"))))

(fn `Place Object`
  (bind _pickedobject (`self.PickedObject`))
  (bind _cube (`/Game/Blueprint/Pickup/BP_Pickup.Cube` _pickedobject))
  (set `/Game/Blueprint/Pickup/BP_Pickup.IsPicked` false _pickedobject)
  (`SceneComponent.K2_DetachFromComponent` _cube "KeepWorld" "KeepWorld" "KeepWorld" true)
  (`PrimitiveComponent.SetSimulatePhysics` _cube true)
  (`PrimitiveComponent.SetCollisionEnabled` _cube "QueryAndPhysics")
  (set `self.PickedObject` null))